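; Data-driven interactable item that configures its mesh, physics, interaction type and hint/phrase data from a DT_InteractableActor row at construction and BeginPlay.
; Player overlap toggles an overlay material and prompt widget.
; Interact dispatches by type: physics grab to the camera with drop/throw, lever toggling a wall lamp and notifying BP_LampPuzzleManager, equip, or inspect.
; Inspect shows a timed text popup, and collectables also report memory fragment phrase data.
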(event `self.ReceiveBeginPlay`
  ; 초기 설정
  (bind _returnvalue (`|GetDataTableRow` "/Game/InteractableActor/New/DT_InteractableActor.DT_InteractableActor" (`self.ItemName`))
    (:`then`
      (bind _output_get (set `self.InteractableActor` _returnvalue))
      (`self.SetItemData` _output_get)
      (`self.SetItemInteraction` _output_get)
      (`self.SetItemPhysics` _output_get)
      (`self.SetItemAction` _output_get)
      (`self.SetItemHint` _output_get)
      (`self.SetItemPhraseData` _output_get))))

(event `self.ReceiveActorBeginOverlap`
  (params (OtherActor :type "Actor Object Reference"))
  ; 상호작용 UI
  (if (`self.Is Interactable`)
    (if (`GameplayStatics.ObjectIsA` OtherActor "/Game/ThirdPerson/Blueprints/BP_ThirdPersonCharacter.BP_ThirdPersonCharacter_C")
      (switch `/Game/InteractableActor/New/EN_UIType` (`self.UIType`)
        (:`NewEnumerator0`
          (`self.ShowUI`)))
      (else
        (`self.HideUI` :!label _label)))))

(event `self.ReceiveActorEndOverlap`
  (params (OtherActor :type "Actor Object Reference"))
  ; 상호작용 UI
  (goto _label))

(event `/Game/InteractableActor/New/BPI_Interaction.Interact`
  (params (Actor :type "Character Object Reference") (Interactor :type "/Game/ThirdPerson/Blueprints/BP_ThirdPersonCharacter Object Reference"))
  ; 상호작용 이벤트
  (set `self.Interactor` Interactor)
  (switch `/Game/InteractableActor/New/EN_InteractionType` (`self.Interaction Type`)
    (:`NewEnumerator0`
      (`self.Grab`))
    (:`NewEnumerator1`
      (`self.Use`))
    (:`NewEnumerator2`
      (`self.Equip`))
    (:`NewEnumerator3`
      (if (`self.isCollectable`)
        (`self.OnMemoryFragmentCollected` self (`.ST_PhraseData_17_82D15756425A90FFC4260F94906159E1` (break `/Game/InteractableActor/New/ST_InteractableActor` (`self.InteractableActor`))))
        (message `/Game/InteractableActor/New/BPI_Interaction.Inspect` self)
        (`self.Inspect`)
        (else
          (`self.Inspect`))))))

(event `/Game/InteractableActor/New/BPI_Interaction.Drop`
  (bind _staticmesh (`self.StaticMesh`))
  ; 아이템 드롭
  (if (`|EnumEquality` (`self.Interaction Type`) "NewEnumerator0")
    (set `self.isGrabbed` false)
    (`self.K2_DetachFromActor` "KeepWorld" "KeepWorld" "KeepWorld")
    (`PrimitiveComponent.SetMassOverrideInKg` _staticmesh "None" (`self.Weight`) true)
    (`PrimitiveComponent.SetSimulatePhysics` _staticmesh true)
    (`PrimitiveComponent.SetEnableGravity` _staticmesh true)
    (set `self.isDropped` true)
    (set `/Game/ThirdPerson/Blueprints/BP_ThirdPersonCharacter.isHoldingItem` false (`self.Interactor`))))

(event `/Game/InteractableActor/New/BPI_Interaction.Throw`
  (bind _staticmesh (`self.StaticMesh`))
  ; 아이템 던지기
  (if (`self.isGrabbed`)
    (`self.K2_DetachFromActor` "KeepWorld" "KeepWorld" "KeepWorld")
    (set `self.isGrabbed` false)
    (`PrimitiveComponent.SetSimulatePhysics` _staticmesh true)
    (`PrimitiveComponent.SetEnableGravity` _staticmesh true)
    (`PrimitiveComponent.AddImpulse` (`self.StaticMesh`) (* (`SceneComponent.GetForwardVector` (`/Game/ThirdPerson/Blueprints/BP_ThirdPersonCharacter.FollowCamera` (`self.Interactor`))) (`self.ThrowStrength`)) "None" true)
    (set `self.isDropped` true)
    (set `/Game/ThirdPerson/Blueprints/BP_ThirdPersonCharacter.isHoldingItem` false (`self.Interactor`))))

(event `/Game/InteractableActor/New/BPI_Interaction.Popup`
  (if (or (`self.Is Key Item`) (`self.Is Hint Item`))
    (`KismetSystemLibrary.PrintString` "It's key or hint item")))

(event `/Game/InteractableActor/New/BPI_Interaction.Grab`
  (bind _staticmesh (`self.StaticMesh`))
  ; 아이템 잡기
  (if (`|EnumEquality` (`self.Interaction Type`) "NewEnumerator0")
    (if (not (`self.isGrabbed`))
      (set `self.isGrabbed` true)
      (set `self.isDropped` false)
      (`PrimitiveComponent.SetSimulatePhysics` _staticmesh false)
      (`PrimitiveComponent.SetEnableGravity` _staticmesh false)
      (`SceneComponent.K2_AttachToComponent` (`self.StaticMesh`) (`/Game/ThirdPerson/Blueprints/BP_ThirdPersonCharacter.FollowCamera` (`self.Interactor`)) "None" "KeepWorld" "KeepWorld" "KeepWorld" false)
      (set `/Game/ThirdPerson/Blueprints/BP_ThirdPersonCharacter.isHoldingItem` true (`self.Interactor`)))))

(event `/Game/InteractableActor/New/BPI_Interaction.ShowUI`
  ; UI 표시 / 숨김
  (`PrimitiveComponent.SetMaterial` (`self.StaticMesh`) 0 "/Game/Materials/PostProcess/MAT_Overlay.MAT_Overlay")
  (`SceneComponent.SetVisibility` (`self.Widget`) true false))

(event `/Game/InteractableActor/New/BPI_Interaction.HideUI`
  ; UI 표시 / 숨김
  (`PrimitiveComponent.SetMaterial` (`self.StaticMesh`) 0 null)
  (`SceneComponent.SetVisibility` (`self.Widget`) false false))

(event `/Game/InteractableActor/New/BPI_Interaction.Use`
  ; 아이템 사용
  (if (`self.isLeverOn`)
    (`self.K2_SetActorRotation` (`KismetMathLibrary.MakeRotator` (.roll (`self.K2_GetActorRotation`)) (`self.MaxPitch`) (.yaw (`self.K2_GetActorRotation`))) true)
    (set `self.isLeverOn` false)
    (`/Game/LevelDecos/Lamp/BP_WallLamp.Set Lamp Off` (`self.BP_WallLamp`))
    (bind _outactors (`GameplayStatics.GetAllActorsOfClass` "/Game/LevelDecos/LeverSwitch/BP_LampPuzzleManager.BP_LampPuzzleManager_C"))
    (`/Game/LevelDecos/LeverSwitch/BP_LampPuzzleManager.CheckPuzzle` (`|GetArrayItem` _outactors))
    (else
      (`self.K2_SetActorRotation` (`KismetMathLibrary.MakeRotator` (.roll (`self.K2_GetActorRotation`)) (`self.MinPitch`) (.yaw (`self.K2_GetActorRotation`))) true)
      (set `self.isLeverOn` true)
      (`/Game/LevelDecos/Lamp/BP_WallLamp.Set Lamp On` (`self.BP_WallLamp`))
      (bind _outactors_2 (`GameplayStatics.GetAllActorsOfClass` "/Game/LevelDecos/LeverSwitch/BP_LampPuzzleManager.BP_LampPuzzleManager_C"))
      (`/Game/LevelDecos/LeverSwitch/BP_LampPuzzleManager.CheckPuzzle` (`|GetArrayItem` _outactors_2)))))

(event `/Game/InteractableActor/New/BPI_Interaction.Inspect`
  ; 아이템 탐색
  (if (and (`self.Is Interactable`) (`self.isInspectable`))
    (if (`self.Is Activated`)
      (bind _returnvalue (`|CreateWidget` "/Game/UI/WB_Popup.WB_Popup_C"))
      (bind _output_get (set `self.PopupUI` _returnvalue))
      (`TextBlock.SetText` (`/Game/UI/WB_Popup.TextBox` _output_get) (`self.UIText`))
      (`UserWidget.AddToViewport` _output_get 0)
      (set `self.Is Activated` false)
      (`KismetSystemLibrary.Delay` 1.2)
      (`Widget.RemoveFromParent` (`self.PopupUI`))
      (else
        (`Widget.SetVisibility` (`self.PopUpUI`) "Hidden")
        (set `self.Is Activated` true)))))

(fn `SetItemAction`
  (params (ST_InteractableActor :type "/Game/InteractableActor/New/ST_InteractableActor Structure"))
  (set `self.Interaction Type` (`.InteractionType_3_0B2CDEE3415BE6D7811A8B80C6C1AE80` (break `/Game/InteractableActor/New/ST_ActionData` (`.ST_ActionData_14_DF6B3C1F4C7CC6A25551D8867E978757` (break `/Game/InteractableActor/New/ST_InteractableActor` ST_InteractableActor))))))

(fn `SetItemData`
  (params (ST_InteractableActor :type "/Game/InteractableActor/New/ST_InteractableActor Structure"))
  (bind _output_get (set `self.Item Static Mesh` (`.ItemStaticMesh_12_81FFC4F343D9A665F8115981124A1AEE` (break `/Game/InteractableActor/New/ST_ItemInfoData` (`.ST_ItemInfoData_10_0B2CDEE3415BE6D7811A8B80C6C1AE80` (break `/Game/InteractableActor/New/ST_InteractableActor` ST_InteractableActor))))))
  (`StaticMeshComponent.SetStaticMesh` (`self.StaticMesh`) _output_get))

(fn `SetItemHint`
  (params (ST_InteractableActor :type "/Game/InteractableActor/New/ST_InteractableActor Structure"))
  (bind (_isuipopupitem _canchangematerial _uitext _uitype) (break `/Game/InteractableActor/New/ST_HintData` (`.ST_HintData_12_C5344FDC4F38427CD1B945A6D072A9B6` (break `/Game/InteractableActor/New/ST_InteractableActor` ST_InteractableActor))))
  (set `self.Is UIPop Up Item` _isuipopupitem)
  (set `self.Can Change Material` _canchangematerial)
  (set `self.UIText` _uitext)
  (set `self.UIType` _uitype))

(fn `SetItemInteraction`
  (params (ST_InteractableActor :type "/Game/InteractableActor/New/ST_InteractableActor Structure"))
  (bind ((`isInteractable_5_0B2CDEE3415BE6D7811A8B80C6C1AE80` _isinteractable) (`isKeyItem_7_73C6A4A64C37A1402C82F4BE9FBD5812` _iskeyitem) (`isHintItem_8_BBEC8FBE43E588F0518CD5B5A68E675B` _ishintitem) (`isLeverOn_11_6537C12649EBA5BCA3B8CAA6386049A0` _isleveron)) (break `/Game/InteractableActor/New/ST_InteractableData` (`.ST_InteractableData_11_FA52706E47AF6459F0BA1195B9B4D50A` (break `/Game/InteractableActor/New/ST_InteractableActor` ST_InteractableActor))))
  (set `self.Is Interactable` _isinteractable)
  (set `self.isLeverOn` _isleveron)
  (set `self.Is Key Item` _iskeyitem)
  (set `self.Is Hint Item` _ishintitem))

(fn `SetItemPhraseData`
  (params (ST_InteractableActor :type "/Game/InteractableActor/New/ST_InteractableActor Structure"))
  (bind (_phraseid _orderindex _phrasetext _isactivated _isfake _collectibleitemtype) (break `/Game/InteractableActor/New/ST_PhraseData` (`.ST_PhraseData_17_82D15756425A90FFC4260F94906159E1` (break `/Game/InteractableActor/New/ST_InteractableActor` ST_InteractableActor))))
  (set `self.Phrase ID` _phraseid)
  (set `self.Order Index` _orderindex)
  (set `self.Phrase Text` _phrasetext)
  (set `self.Is Activated` _isactivated)
  (set `self.Is Fake` _isfake)
  (set `self.Collectible Item Type` _collectibleitemtype))

(fn `SetItemPhysics`
  (params (ST_InteractableActor :type "/Game/InteractableActor/New/ST_InteractableActor Structure"))
  (bind _output_get (set `self.Weight` (`.Weight_7_E034D519482AEFFFCDB13785F6E24C29` (break `/Game/InteractableActor/New/ST_PhysicsData` (`.ST_PhysicsData_13_69EB9A3040D4A2B09C18D9AC2139E7E5` (break `/Game/InteractableActor/New/ST_InteractableActor` ST_InteractableActor))))))
  (`PrimitiveComponent.SetMassOverrideInKg` (`self.StaticMesh`) "None" _output_get true))

(fn `SetItemVisual`
  (params (ST_InteractableActor :type "/Game/InteractableActor/New/ST_InteractableActor Structure"))
  (bind (_isuipopupitem _canchangematerial _uitext _uitype) (break `/Game/InteractableActor/New/ST_HintData` (`.ST_HintData_12_C5344FDC4F38427CD1B945A6D072A9B6` (break `/Game/InteractableActor/New/ST_InteractableActor` ST_InteractableActor))))
  (set `self.Is UIPop Up Item` _isuipopupitem)
  (set `self.Can Change Material` _canchangematerial)
  (set `self.UIType` _uitype))

(fn `UserConstructionScript`
  (bind _returnvalue (`|GetDataTableRow` "/Game/InteractableActor/New/DT_InteractableActor.DT_InteractableActor" (`self.ItemName`))
    (:`then`
      (bind _output_get (set `self.InteractableActor` _returnvalue))
      (`self.SetItemData` _output_get)
      (`self.SetItemInteraction` _output_get)
      (`self.SetItemPhysics` _output_get)
      (`self.SetItemAction` _output_get)
      (`self.SetItemHint` _output_get)
      (`self.SetItemPhraseData` _output_get))))